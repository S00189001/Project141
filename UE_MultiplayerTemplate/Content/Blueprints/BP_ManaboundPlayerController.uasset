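; Player controller for Manabound that routes player input to the in-game UI, chat and action bar abilities.
; BeginPlay has the game mode load the UI, while input handlers open chat, inventory, character sheet, spell book and in-game menu.
; Any key press is matched against action bar slot mappings to cast abilities, and left clicks call LeftMouseClicked.
; Chat messages go through the game mode to everyone, and AddMessageToChat writes them into the HUD.
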(event `CreatePlayerHud`
  (bind _returnvalue (`|CreateWidget` "/Game/InGameUI/UMG_HeadsUpDisplay.UMG_HeadsUpDisplay_C" (`GameplayStatics.GetPlayerController` 0)))
  (bind _output_get (set `self.HeadsUpDisplay` _returnvalue))
  (`UserWidget.AddToViewport` _output_get 0))

(event `ShowChat`
  (params (Focused :type Boolean))
  (`/Game/InGameUI/UMG_HeadsUpDisplay.setFocusOnChat` (`self.HeadsUpDisplay`) Focused)
  (if Focused
    (`WidgetBlueprintLibrary.SetInputMode_GameAndUIEx` self (`self.HeadsUpDisplay`))
    (else
      (`WidgetBlueprintLibrary.SetInputMode_GameOnly` self))))

(event `Key|Enter`
  (params (Key :type "Key Structure"))
  (:`Pressed`
    (`self.ShowChat` true)))

(event `InputAction|OpenCharacterSheet`
  (params (Key :type "Key Structure"))
  (:`Pressed`
    (`/Game/InGameUI/UMG_HeadsUpDisplay.ToggleCharacterSheet` (`self.HeadsUpDisplay`))))

(event `ServerSendMessage`
  (params (Name :type String) (Message :type String))
  (bind _asmana_bound_game_mode (cast `/Game/Blueprints/ManaBoundGameMode` (`GameplayStatics.GetGameMode`)))
  (`/Game/Blueprints/ManaBoundGameMode.SendMessageToEveryone` _asmana_bound_game_mode Name Message))

(event `AddMessageToChat`
  (params (Name :type String) (Message :type String))
  (`/Game/InGameUI/UMG_HeadsUpDisplay.AddMessageIntoList` (`self.HeadsUpDisplay`) Name Message))

(event `Key|C`
  (params (Key :type "Key Structure"))
  ;[1 1 1] 'C' Show / Hide the players Character Sheet
)

(event `Key|Escape`
  (params (Key :type "Key Structure"))
  (:`Pressed`
    (bind _asmaster_game_instance (cast `MasterGameInstance` (`GameplayStatics.GetGameInstance`)))
    (`MasterGameInstance.InGameLoadMenu` _asmaster_game_instance)))

(event `self.ReceiveBeginPlay`
  ;[1 1 1] EventBeginPlay - Load Player HUDs
  (bind _asmana_bound_game_mode (cast `/Game/Blueprints/ManaBoundGameMode` (`GameplayStatics.GetGameMode`)))
  (`/Game/Blueprints/ManaBoundGameMode.LoadIngameUI` _asmana_bound_game_mode))

(event `Key|LeftMouseButton` :consume false
  (params (Key :type "Key Structure"))
  ;[1 1 1] LMB Listener
  (:`Pressed`
    (`self.LeftMouseClicked`)))

(event `Key|RightMouseButton`
  (params (Key :type "Key Structure")))

(event `InputAction|OpenInventory`
  (params (Key :type "Key Structure"))
  (:`Pressed`
    (`/Engine/EditorBlueprintResources/StandardMacros.IsValid` (`self.InventoryWidget`)
      (:`Is Valid`
        _)
      (:`Is Not Valid`
        (bind _returnvalue (`|CreateWidget` "/Game/InGameUI/InvetorySystem/WP_Invetory.WP_Invetory_C"))
        (set `self.InventoryWidget` _returnvalue)))
    (`UserWidget.AddToViewport` (`self.InventoryWidget`) 0)))

(event `Key|Tab`
  (params (Key :type "Key Structure"))
  ;[1 1 1] 'TAB' Show / Hide the players Spell Book
  (:`Pressed`
    (bind _isa (`/Engine/EditorBlueprintResources/StandardMacros.FlipFlop`)
      (:`A`
        (bind _asmana_bound_game_mode (cast `/Game/Blueprints/ManaBoundGameMode` (`GameplayStatics.GetGameMode`)))
        (bind _umg_spellbook (`/Game/InGameUI/UMG_HeadsUpDisplay.UMG_SpellBook` (`/Game/Blueprints/ManaBoundGameMode.InGameHeadsUpDisplay` _asmana_bound_game_mode)))
        (`Widget.SetVisibility` _umg_spellbook "Visible"))
      (:`B`
        (`Widget.SetVisibility` _umg_spellbook "Hidden")))
    (set `self.bShowMouseCursor` _isa)))

(event `Key|AnyKey` :consume false
  (params (Key :type "Key Structure"))
  (:`Pressed`
    (`self.CheckBindings` Key)))

(fn `CheckBindings`
  (params (Key :type "Key Structure" :default "None"))
  (for _array_element (`PanelWidget.GetAllChildren` (`/Game/InGameUI/ActionBar/UMG_ActionBar.AbilitySlotContainer` (`/Game/InGameUI/UMG_HeadsUpDisplay.UMG_ActionBar` (`self.HeadsUpDisplay`))))
    (bind _asumg_action_bar_slot (cast `/Game/InGameUI/ActionBar/UMG_ActionBarSlot` _array_element))
    (if (== (`/Game/InGameUI/ActionBar/UMG_ActionBarSlot.Mapping` _asumg_action_bar_slot) (`local.Key`))
      (`/Game/InGameUI/ActionBar/UMG_ActionBarSlot.CastAbility` _asumg_action_bar_slot))))

(fn `DisableMouse`
  (set `self.bShowMouseCursor` false)
  (`WidgetBlueprintLibrary.SetInputMode_GameAndUIEx` (`GameplayStatics.GetPlayerController` 0) null))

(fn `EnableLMBClickChecks`)

(fn `EnableMouse`
  (set `self.bShowMouseCursor` true)
  (bind _asmana_bound_game_mode (cast `/Game/Blueprints/ManaBoundGameMode` (`GameplayStatics.GetGameMode`)))
  (`WidgetBlueprintLibrary.SetInputMode_GameAndUIEx` (`GameplayStatics.GetPlayerController` 0) (`/Game/Blueprints/ManaBoundGameMode.InGameHeadsUpDisplay` _asmana_bound_game_mode))
  (`self.SetIgnoreMoveInput` true))

(fn `UserConstructionScript`)