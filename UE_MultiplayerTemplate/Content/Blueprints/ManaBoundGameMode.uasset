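; ManaBoundGameMode is the game mode that tracks connected players, relays chat, builds the in-game HUD and respawns killed players.
; PostLogin stores each BP_ManaboundPlayerController in a Players array, which SendMessageToEveryone loops over to push chat messages.
; LoadIngameUI creates the HUD widget for player index 0 and sets that player's HUD and compass visible.
; OnPlayerKilled unpossesses the killed player's controller and calls RestartPlayer on it.
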(event `self.K2_PostLogin`
  (params (NewPlayer :type "PlayerController Object Reference"))
  (bind _asbp_manabound_player_controller (cast `/Game/Blueprints/BP_ManaboundPlayerController` NewPlayer))
  (`KismetArrayLibrary.Array_Add` (`self.Players`) _asbp_manabound_player_controller))

(event `SendMessageToEveryone`
  (params (Name :type String) (Message :type String))
  (for _array_element (`self.Players`)
    (`/Game/Blueprints/BP_ManaboundPlayerController.AddMessageToChat` _array_element Name Message)))

(event `LoadIngameUI`
  (bind _returnvalue (`GameplayStatics.GetPlayerController` 0))
  (bind _returnvalue_2 (`|CreateWidget` "/Game/InGameUI/UMG_HeadsUpDisplay.UMG_HeadsUpDisplay_C" _returnvalue))
  (bind _output_get (set `self.InGameHeadsUpDisplay` _returnvalue_2))
  (`UserWidget.AddToViewport` _output_get 0)
  (bind _asbp_manabound_player_controller (cast `/Game/Blueprints/BP_ManaboundPlayerController` _returnvalue))
  (set `/Game/Blueprints/BP_ManaboundPlayerController.HUDVisibility` "Visible" _asbp_manabound_player_controller)
  (bind _asthird_person_character (cast `/Game/ThirdPersonCPP/Blueprints/ThirdPersonCharacter` (`GameplayStatics.GetPlayerCharacter` 0)))
  (set `/Game/ThirdPersonCPP/Blueprints/ThirdPersonCharacter.CompassVisibility` "Visible" _asthird_person_character))

(fn `OnPlayerKilled`
  (params (Player :type "Character Object Reference"))
  (locals (Controller :type "Controller Object Reference"))
  (bind _output_get (set `local.Controller` (`Pawn.GetController` Player)))
  (`Controller.UnPossess` _output_get)
  (`self.RestartPlayer` (`local.Controller`)))

(fn `UserConstructionScript`)