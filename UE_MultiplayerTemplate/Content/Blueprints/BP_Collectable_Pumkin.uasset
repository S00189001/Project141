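; Pumpkin collectable actor that the player consumes with the E key to restore hunger and thirst.
; The key press plays a sound, then applies Gameplay Ability System restore effects to player 0's ThirdPersonCharacter.
; Attribute checks above 100 apply max-hunger and max-thirst effects, apparently as a cap.
; Pickup then goes through a server event to a multicast that destroys the actor; no overlap logic is active here.
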(event `Key|E`
  (params (Key :type "Key Structure"))
  (:`Pressed`
    (`GameplayStatics.PlaySound2D` "/Engine/VREditor/Sounds/UI/Foliage_Placed.Foliage_Placed" 1.0 1.0 0.0 null null)
    (bind _asthird_person_character (cast `/Game/ThirdPersonCPP/Blueprints/ThirdPersonCharacter` (`GameplayStatics.GetPlayerCharacter` 0)))
    (bind _abilitysystemcomponent (`UE_MultiplayerTempCharacter.AbilitySystemComponent` _asthird_person_character))
    (`AbilitySystemComponent.BP_ApplyGameplayEffectToSelf` :`self` _abilitysystemcomponent :`GameplayEffectClass` "/Game/AbilitiesSystem/GameplayEffects/GE_RestoreHunger.GE_RestoreHunger_C" :`Level` 1.0)
    (`AbilitySystemComponent.BP_ApplyGameplayEffectToSelf` :`self` _abilitysystemcomponent :`GameplayEffectClass` "/Game/AbilitiesSystem/GameplayEffects/BP_RestoreThirst.BP_RestoreThirst_C" :`Level` 1.0)
    (if (> (`.ReturnValue` (`AbilitySystemBlueprintLibrary.GetFloatAttributeFromAbilitySystemComponent` _abilitysystemcomponent (struct :`AttributeName` "Hunger" :`Attribute` "/Script/UE_MultiplayerTemp.GASAttributeSet:Hunger"))) 100.0)
      (`AbilitySystemComponent.BP_ApplyGameplayEffectToSelf` :`self` _abilitysystemcomponent :`GameplayEffectClass` "/Game/AbilitiesSystem/GameplayEffects/GE_MaxHunger.GE_MaxHunger_C" :`Level` 1.0))
    (if (> (`.ReturnValue` (`AbilitySystemBlueprintLibrary.GetFloatAttributeFromAbilitySystemComponent` _abilitysystemcomponent (struct :`AttributeName` "Thirst" :`Attribute` "/Script/UE_MultiplayerTemp.GASAttributeSet:Thirst"))) 100.0)
      (`AbilitySystemComponent.BP_ApplyGameplayEffectToSelf` :`self` _abilitysystemcomponent :`GameplayEffectClass` "/Game/AbilitiesSystem/GameplayEffects/BP_MaxThirst.BP_MaxThirst_C" :`Level` 1.0))
    (`self.Server_ItemPickedUp`)))

(event `Server_ItemPickedUp`
  (`self.Multicast_ItemPickedUp`))

(event `Multicast_ItemPickedUp`
  (`self.K2_DestroyActor` self))

(fn `UserConstructionScript`
  (`parent.UserConstructionScript`))