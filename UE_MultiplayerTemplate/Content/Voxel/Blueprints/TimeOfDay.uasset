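; Day/night cycle actor that rotates the level's directional light and refreshes BP_Sky_Sphere to match.
; At BeginPlay it finds both actors, and the authority seeds ServerTime from ManaBoundGameMode's start time; clients copy it, also through its OnRep.
; Each machine then advances time locally by a fixed step per tick, without delta-time scaling.
; Hour thresholds switch the sun between white, warm orange and black light.
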(event `self.ReceiveBeginPlay`
  (`KismetSystemLibrary.Delay` 0.2)
  (bind _outactors (`GameplayStatics.GetAllActorsOfClass` "/Script/Engine.DirectionalLight"))
  (if (> (`KismetArrayLibrary.Array_Length` _outactors) 0)
    (set `self.Sun` (`|GetArrayItem` _outactors))
    (bind _outactors_2 (`GameplayStatics.GetAllActorsOfClass` "/Engine/EngineSky/BP_Sky_Sphere.BP_Sky_Sphere_C"))
    (if (> (`KismetArrayLibrary.Array_Length` _outactors_2) 0)
      (set `self.Sky Sphere` (`|GetArrayItem` _outactors_2))
      (`/Engine/EditorBlueprintResources/ActorMacros.Switch Has Authority`
        (:`Authority`
          (bind _output_get (set `self.Server Time` (`/Game/Blueprints/ManaBoundGameMode.SunStartTime` (cast `/Game/Blueprints/ManaBoundGameMode` (`GameplayStatics.GetGameMode`) :!pure true))))
          (set `self.Current Time` _output_get))
        (:`Remote`
          (set `self.Current Time` (`self.Server Time`)))))))

(event `self.ReceiveTick`
  (params (DeltaSeconds :type "Float (single-precision)"))
  (bind _time_of_day (`self.Time Of Day`))
  (bind _time_of_day_2 (`self.Time Of Day`))
  (set `self.Current Time` (+ (/ 24.0 (`self.CycleDuration`)) (`self.Current Time`)))
  (bind _output_get (set `self.Time Of Day` (mod (`self.Current Time`) 24.0)))
  (set `self.DayCompletePercentage` (/ _output_get 24.0))
  (bind _sun (`self.Sun`)
    (:`then`
      (`self.K2_SetActorRotation` _sun (`KismetMathLibrary.MakeRotator` 180.0 (- (* (`self.DayCompletePercentage`) 360.0) 180.0) 150.0) false)
      (`/Engine/EngineSky/BP_Sky_Sphere.UpdateSunDirection` (`self.Sky Sphere`))
      (if (or (< _time_of_day_2 2.0) (> _time_of_day_2 10.5))
        (`LightComponent.SetIntensity` (`Light.LightComponent` (`self.Sun`)) 1.75)
        (`LightComponent.SetLightColor` (`Light.LightComponent` (`self.Sun`)) (struct :`R` 1.0 :`G` 0.348223 :`B` 0.054605 :`A` 1.0) true)
        (if (and (> _time_of_day 15.0) (< _time_of_day 21.0))
          (`LightComponent.SetLightColor` (`Light.LightComponent` (`self.Sun`)) (struct :`A` 1.0) true)
          (`LightComponent.SetIntensity` (`Light.LightComponent` (`self.Sun`)) 1.75))
        (else
          (`LightComponent.SetIntensity` (`Light.LightComponent` (`self.Sun`)) 2.0)
          (`LightComponent.SetLightColor` (`Light.LightComponent` (`self.Sun`)) (struct :`R` 1.0 :`G` 1.0 :`B` 1.0 :`A` 1.0) true))))
    (:`else`)))

(fn `OnRep_Server Time`
  (set `self.Current Time` (`self.Server Time`)))

(fn `UserConstructionScript`)