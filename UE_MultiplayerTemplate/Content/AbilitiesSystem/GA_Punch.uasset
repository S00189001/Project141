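; GA_Punch is a Gameplay Ability that performs a melee punch and damages the target it hits.
; Activation plays the attack montage while waiting once for a Weapon.Hit gameplay event, whose target data receives the damage Gameplay Effect.
; The ability ends when the montage completes, blends out or is interrupted.
; The stored event-wait task is explicitly ended on ability end so the listener does not linger.
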(event `self.K2_ActivateAbility`
  (bind (_returnvalue_owneractor _returnvalue_avataractor _returnvalue_playercontroller _returnvalue_abilitysystemcomponent _returnvalue_skeletalmeshcomponent) (break `GameplayAbilityActorInfo` (`self.GetActorInfo`)))
  ;[1 1 1] Punch Ability
  (`|PlayMontage` _returnvalue_skeletalmeshcomponent "/Game/AbilitiesSystem/Animations/M_Attack.M_Attack"
    (:`then`
      (bind (_asynctaskproxy _payload) (`AbilityTask_WaitGameplayEvent.WaitGameplayEvent` (struct :`TagName` "Weapon.Hit") null true)
        (:`then`
          ;[1 1 1] Async to Cleanup
          (set `self.Async Task` _asynctaskproxy))
        (:`EventReceived`
          (`self.BP_ApplyGameplayEffectToTarget` (`.TargetData` (break `GameplayEventData` _payload)) "/Game/AbilitiesSystem/GE_Damage.GE_Damage_C"))))
    (:`OnCompleted`
      (`self.K2_EndAbility` :!label _label))
    (:`OnBlendOut`
      (goto _label))
    (:`OnInterrupted`
      (goto _label))))

(event `self.K2_OnEndAbility`
  (params (bWasCancelled :type Boolean))
  (bind _async_task (`self.Async Task`))
  ;[1 1 1] Cleanup Async Task
  (`/Engine/EditorBlueprintResources/StandardMacros.IsValid` _async_task
    (:`Is Valid`
      (`GameplayTask.EndTask` _async_task))))