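; Projectile ability actor that animates the player's cast and launches itself in step with the animation.
; BeginPlay starts the fireball montage on the player character's mesh, and CastAbility replays it from its EndCast section.
; A montage notify during that section calls ActivateEffect, which activates the ProjectileMovement component.
; Each of these events extends parent class logic, and this child adds no overlap or tick behavior.
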(event `self.ReceiveBeginPlay`
  (`parent.ReceiveBeginPlay`)
  (`|PlayMontage` (`Character.Mesh` (`self.Player Character Ref`)) "/Game/AbilitiesSystem/Animations/MixamoAnimations/ProMagePack/Fireball_014UE4_Montage.Fireball_014UE4_Montage"))

(event `self.CastAbility`
  ;[1 1 1] Runs Parent Code then calls Activate Effect
  (`parent.CastAbility`)
  (`|PlayMontage` (`Character.Mesh` (`self.Player Character Ref`)) "/Game/AbilitiesSystem/Animations/MixamoAnimations/ProMagePack/Fireball_014UE4_Montage.Fireball_014UE4_Montage" 1.0 0.0 "EndCast"
    (:`OnNotifyBegin`
      (`self.ActivateEffect`))))

(event `self.ActivateEffect`
  ;[1 1 1] Runs Parent Code then Toggles Projectile Activation
  (`parent.ActivateEffect`)
  (`ActorComponent.Activate` (`self.ProjectileMovement`) false))

(fn `UserConstructionScript`
  (`parent.UserConstructionScript`))