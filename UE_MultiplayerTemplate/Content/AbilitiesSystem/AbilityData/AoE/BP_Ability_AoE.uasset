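; Area-of-effect ability actor that plays a cast montage on the player character and places its particle effect on the ground beneath them.
; CastAbility plays the montage, and its notify begin calls ActivateEffect.
; ActivateEffect starts the particle system, zeroes the actor's rotation and moves it to the hit location of a downward visibility trace from the player.
; Both events extend parent ability logic, and no damage or overlap handling is implemented here.
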(event `self.CastAbility`
  (`parent.CastAbility`)
  (`|PlayMontage` (`Character.Mesh` (`self.Player Character Ref`)) "/Game/AbilitiesSystem/Animations/MixamoAnimations/ProMagePack/AoE_014UE4_Montage.AoE_014UE4_Montage"
    (:`OnNotifyBegin`
      (`self.ActivateEffect`))))

(event `self.ActivateEffect`
  (bind _returnvalue (`GameplayStatics.GetPlayerCharacter` 0))
  (bind _returnvalue_2 (`self.K2_GetActorLocation` _returnvalue))
  (`parent.ActivateEffect`)
  (`ActorComponent.Activate` (`self.ParticleSystem`) false)
  (`self.K2_SetActorRotation` (struct))
  (bind _outhit (`KismetSystemLibrary.LineTraceSingle` _returnvalue_2 (+ _returnvalue_2 (0.0 0.0 -10000.0)) "TraceTypeQuery1" false (`|MakeArray` _returnvalue :!type "Actor Object Reference")))
  (`self.K2_SetActorLocation` (`.Location` (`GameplayStatics.BreakHitResult` _outhit))))

(fn `UserConstructionScript`
  (`parent.UserConstructionScript`))