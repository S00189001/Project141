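; Healing Spirit area-of-effect ability actor that periodically heals characters standing inside it.
; On BeginPlay it shows its decal, sets its lifespan and starts a looping timer at the DoT interval.
; Each tick applies GE_HealPlayer through the ability system component of every ThirdPersonCharacter overlapping AbilityRoot.
; The loop's completion also leads into the heal node, adding one application after each pass.
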(event `self.ReceiveBeginPlay`
  (`parent.ReceiveBeginPlay`)
  (`SceneComponent.SetVisibility` (`self.Decal`) true false)
  (`self.SetLifeSpan` (`self.LifeSpan`))
  (`KismetSystemLibrary.K2_SetTimerDelegate` (delegate `TickEffect`) (`self.DoTTimer`) true))

(event `TickEffect`
  (for _array_element (`PrimitiveComponent.GetOverlappingActors` (`self.AbilityRoot`) "/Game/ThirdPersonCPP/Blueprints/ThirdPersonCharacter.ThirdPersonCharacter_C")
    (`AbilitySystemComponent.BP_ApplyGameplayEffectToSelf` :`self` (`AbilitySystemBlueprintLibrary.GetAbilitySystemComponent` _array_element) :`GameplayEffectClass` "/Game/AbilitiesSystem/GameplayEffects/GE_HealPlayer.GE_HealPlayer_C" :!label _label))
  (goto _label))

(fn `UserConstructionScript`
  (`parent.UserConstructionScript`))