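; BP_Ability is an ability actor that starts casting as soon as it spawns.
; On BeginPlay it gets the HUD from ManaBoundGameMode, then either shows a cast bar and binds to its CastSuccessful event, or casts immediately when AbilityDetails has no cast time.
; CastAbility only prints a debug string, while InterruptCast destroys the actor and prints a message.
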(event `self.ReceiveBeginPlay`
  (bind _asmana_bound_game_mode (cast `/Game/Blueprints/ManaBoundGameMode` (`GameplayStatics.GetGameMode`)))
  (set `self.LocInGameHeadsUpDisplay` (`/Game/Blueprints/ManaBoundGameMode.InGameHeadsUpDisplay` _asmana_bound_game_mode))
  (`self.BeginCasting`))

(fn `BeginCasting`
  (bind (_abilitydetails_name _abilitydetails_description _abilitydetails_manacost _abilitydetails_staminacost _abilitydetails_cooldown _abilitydetails_casttime) (break `/Game/AbilitiesSystem/AbilityData/Struct_AbilityData` (`self.AbilityDetails`)))
  (if (> _abilitydetails_casttime 0.0)
    (bind _castbarref (`/Game/InGameUI/UMG_HeadsUpDisplay.DisplayCastBar` (`self.LocInGameHeadsUpDisplay`) self))
    (add `/Game/InGameUI/ActionBar/UMG_Castbar.CastSuccessful` _castbarref (`|CreateDelegate` :!event `CastAbility`))
    (else
      (`self.CastAbility`))))

(fn `CastAbility`
  (`KismetSystemLibrary.PrintString` "Casted Ability"))

(fn `InterruptCast`
  (`self.K2_DestroyActor`)
  (`KismetSystemLibrary.PrintString` "Interrupt"))

(fn `UserConstructionScript`)