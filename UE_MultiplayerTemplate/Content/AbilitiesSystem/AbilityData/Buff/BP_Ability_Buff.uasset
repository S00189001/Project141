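; Base ability actor for timed buffs: on spawn it destroys same-class actors attached to the caster, then plays a player cast montage.
; CastAbility sets the lifespan, plays a sound, adds the buff to the HUD buff panel and starts a looping tick timer.
; TickBuff and ClearBuff are empty here, and EndPlay calls BuffRemoved when the buff ends.
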(event `self.ReceiveBeginPlay`
  (`self.ClearDuplicates`)
  (`parent.ReceiveBeginPlay`)
  (`|PlayMontage` (`Character.Mesh` (`self.Player Character Ref`)) "/Game/AbilitiesSystem/Animations/MixamoAnimations/ProMagePack/AoE_014UE4_Montage.AoE_014UE4_Montage"))

(event `self.CastAbility`
  (`self.SetLifeSpan` (`self.BuffLifespan`))
  (`self.Apply Buff`)
  (bind _returnvalue (`KismetSystemLibrary.K2_SetTimerDelegate` (delegate `TickBuff`) (`self.BuffTickRate`) true))
  (set `self.BuffTickTimer` _returnvalue))

(event `TickBuff`)

(event `self.ReceiveEndPlay`
  (params (EndPlayReason :type "EEndPlayReason Enum" :default "Destroyed"))
  (`self.BuffRemoved`))

(fn `Apply Buff`
  (`GameplayStatics.PlaySound2D` "/Engine/VREditor/Sounds/UI/Enter_Simulate.Enter_Simulate" 1.0 1.0 0.0 null null)
  (bind _asbp_manabound_game_state (cast `/Game/Blueprints/BP_ManaboundGameState` (`GameplayStatics.GetGameState`)))
  (`/Game/InGameUI/Buffs/UMG_BuffPanel.AddBuffToUI` (`/Game/InGameUI/UMG_HeadsUpDisplay.UMG_BuffPanel` (`/Game/Blueprints/BP_ManaboundGameState.HeadsUpDisplay` _asbp_manabound_game_state)) self))

(fn `ClearBuff`)

(fn `ClearDuplicates`
  (for _array_element (`self.GetAttachedActors` (`self.Caster`) true)
    (if (== (`GameplayStatics.GetObjectClass` _array_element) (`GameplayStatics.GetObjectClass` self))
      (`self.K2_DestroyActor` _array_element))))

(fn `UserConstructionScript`
  (`parent.UserConstructionScript`))