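; Gameplay ability that buffs the owner's attack power, timed to a casting montage.
; Activation calls a multicast event that plays the montage and waits once for the Magic.Buff.AttackPower gameplay event, then applies GE_BuffAttackPower to the owner.
; The ability ends when the montage completes, blends out or is interrupted.
; The event-wait task is stored and explicitly ended in OnEndAbility to clean up the listener.
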(event `self.K2_ActivateAbility`
  (`self.Multicast_GA_BuffAttackPower`))

(event `Multicast_GA_BuffAttackPower`
  (bind (_returnvalue_owneractor _returnvalue_avataractor _returnvalue_playercontroller _returnvalue_abilitysystemcomponent _returnvalue_skeletalmeshcomponent) (break `GameplayAbilityActorInfo` (`self.GetActorInfo`)))
  (`|PlayMontage` _returnvalue_skeletalmeshcomponent "/Game/AbilitiesSystem/Animations/M_BuffAttackPoewer.M_BuffAttackPoewer"
    (:`then`
      (bind _asynctaskproxy (`AbilityTask_WaitGameplayEvent.WaitGameplayEvent` (struct :`TagName` "Magic.Buff.AttackPower") null true)
        (:`then`
          ;[1 1 1] Async To Cleanup
          (set `self.Async Task` _asynctaskproxy))
        (:`EventReceived`
          (`self.BP_ApplyGameplayEffectToOwner` "/Game/AbilitiesSystem/GameplayEffects/GE_BuffAttackPower.GE_BuffAttackPower_C"))))
    (:`OnCompleted`
      (`self.K2_EndAbility` :!label _label))
    (:`OnBlendOut`
      (goto _label))
    (:`OnInterrupted`
      (goto _label))))

(event `self.K2_OnEndAbility`
  (params (bWasCancelled :type Boolean))
  (bind _async_task (`self.Async Task`))
  ;[1 1 1] Cleanup Async Task
  (`/Engine/EditorBlueprintResources/StandardMacros.IsValid` _async_task
    (:`Is Valid`
      (`GameplayTask.EndTask` _async_task))))