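; BP_BookStack procedurally builds decorative book stacks from one instanced static mesh in the construction script.
; StackType selects a horizontal row with random leaning runs, a vertical pile with random yaw, or a row following the spline's length and heading.
; A seeded random stream varies scale, lean and yaw for repeatable results.
; Mesh bounds and trigonometric helpers compute each book's footprint, lift and lean overlap to advance the next placement.
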(fn `CalculateBookWidth`
  (params (Roll :type "Float (double-precision)") (Scale :type "Float (double-precision)"))
  (returns (ZOffset :type "Float (double-precision)") (TotalWidth :type "Float (double-precision)"))
  (locals (_Scale :type "Float (double-precision)" :default 0.0))
  (bind _returnvalue (- 90.0 Roll))
  (return (* (* (`local.Scale`) (`KismetMathLibrary.DegCos` _returnvalue)) (.y (`self.BookSize`))) (* (.y (`self.BookSize`)) (+ (* (`KismetMathLibrary.DegSin` _returnvalue) (`local.Scale`)) (* (`KismetMathLibrary.DegCos` _returnvalue) (/ (.z (`self.BookSize`)) (.y (`self.BookSize`))))))))

(fn `CalculateRoll`
  (params (PreviousRoll :type "Float (double-precision)"))
  (returns (roll :type "Float (double-precision)"))
  (bind _randomstream (`self.RandomStream`))
  (if (`KismetMathLibrary.RandomBoolWithWeightFromStream` (`self.RollChance`) _randomstream)
    (if (> (`KismetMathLibrary.Abs` (`local.PreviousRoll`)) 0.0)
      (return (`local.PreviousRoll`))
      (else
        (return (`KismetMathLibrary.RandomFloatInRangeFromStream` 0.0 (`self.MaxRoll`) _randomstream))))
    (else
      (return 0.0))))

(fn `CalculateRollOffset`
  (params (PreviousRoll :type "Float (double-precision)") (currentRoll :type "Float (double-precision)"))
  (returns (Offset :type "Float (double-precision)"))
  (bind _returnvalue (- 90.0 (`local.PreviousRoll`)))
  (bind _returnvalue_2 (`KismetMathLibrary.DegCos` _returnvalue))
  (if (and (> PreviousRoll 0.0) (> currentRoll 0.0))
    (return (* (- (* _returnvalue_2 (/ (.z (`self.BookSize`)) (.y (`self.BookSize`)))) (* (/ 1.0 (/ (`KismetMathLibrary.DegTan` _returnvalue) (`KismetMathLibrary.DegCos` _returnvalue))) _returnvalue_2)) (.y (`self.BookSize`))))
    (else
      (return 0.0))))

(fn `PlaceHorizontalStack`
  (locals (CurrentIndex :type Integer) (CurrentRoll :type "Float (double-precision)") (CurrentScale :type "Float (double-precision)") (LastLocation :type "Float (double-precision)") (PreviousRoll :type "Float (double-precision)"))
  (bind (_scaleminmax_x _scaleminmax_y) (`KismetMathLibrary.BreakVector2D` (`self.ScaleMinMax`)))
  (bind (_zoffset _totalwidth) (`self.CalculateBookWidth` (`local.CurrentRoll`) (`local.CurrentScale`)))
  (for _index (range (`self.NumberOfBooks`))
    (bind _output_get (set `local.CurrentIndex` _index))
    (set `local.CurrentRoll` (`self.CalculateRoll` (`local.PreviousRoll`)))
    (set `local.CurrentScale` (`KismetMathLibrary.RandomFloatInRangeFromStream` _scaleminmax_x _scaleminmax_y (`self.RandomStream`)))
    (`|ExecutionSequence`
      (:`then_0`
        (`InstancedStaticMeshComponent.AddInstance` (`self.InstancedStaticMesh`) (`KismetMathLibrary.MakeTransform` (`KismetMathLibrary.MakeVector` 0.0 (- (`local.LastLocation`) (`self.CalculateRollOffset` (`local.PreviousRoll`) (`local.CurrentRoll`))) _zoffset) (`KismetMathLibrary.MakeRotator` (`local.CurrentRoll`)) (`KismetMathLibrary.MakeVector` 1.0 (`local.CurrentScale`) 1.0))))
      (:`then_1`
        (set `local.LastLocation` (- (+ _totalwidth (`local.LastLocation`)) (`self.CalculateRollOffset` (`local.PreviousRoll`) (`local.CurrentRoll`))))
        (set `local.PreviousRoll` (`local.CurrentRoll`))))))

(fn `PlaceSplineStack`
  (locals (CurrentIndex :type Integer) (CurrentYaw :type "Float (double-precision)") (CurrentScale :type "Float (double-precision)") (Distance :type "Float (double-precision)") (PreviousYaw :type "Float (double-precision)"))
  (bind (_booksize_x _booksize_y) (`KismetMathLibrary.BreakVector` (`self.BookSize`)))
  (bind (_scaleminmax_x _scaleminmax_y) (`KismetMathLibrary.BreakVector2D` (`self.ScaleMinMax`)))
  (bind (_zoffset _totalwidth) (`self.CalculateBookWidth` (`local.CurrentYaw`) (`local.CurrentScale`)))
  (bind _returnvalue (`SplineComponent.GetTransformAtDistanceAlongSpline` (`self.Spline`) (+ (- (`local.Distance`) (`self.CalculateRollOffset` (`local.PreviousYaw`) (`local.CurrentYaw`))) 0.0) "Local" false))
  (for _index (range (`.ReturnValue` (`KismetMathLibrary.FMod` (`SplineComponent.GetSplineLength` (`self.Spline`)) _booksize_y)))
    (bind _output_get (set `local.CurrentIndex` _index))
    (set `local.CurrentYaw` 0.0)
    (set `local.CurrentScale` (`KismetMathLibrary.RandomFloatInRangeFromStream` _scaleminmax_x _scaleminmax_y (`self.RandomStream`)))
    (`|ExecutionSequence`
      (:`then_0`
        (`InstancedStaticMeshComponent.AddInstance` (`self.InstancedStaticMesh`) (`KismetMathLibrary.MakeTransform` (+ (`KismetMathLibrary.MakeVector` 0.0 0.0 _zoffset) (.location _returnvalue)) (`KismetMathLibrary.MakeRotator` (`local.CurrentYaw`) 0.0 (+ (.yaw (.rotation _returnvalue)) 90.0)) (`KismetMathLibrary.MakeVector` 1.0 (`local.CurrentScale`) 1.0))))
      (:`then_1`
        (set `local.Distance` (+ 0.0 (- (+ _totalwidth (`local.Distance`)) (`self.CalculateRollOffset` (`local.PreviousYaw`) (`local.CurrentYaw`)))))
        (set `local.PreviousYaw` (`local.CurrentYaw`))))))

(fn `PlaceVerticalStack`
  (locals (CurrentIndex :type Integer) (CurrentScale :type "Float (double-precision)") (currentYaw :type "Float (double-precision)" :default 0.0) (LastLocation :type "Float (double-precision)") (CurrentRoll :type "Float (double-precision)"))
  (bind (_scaleminmax_x _scaleminmax_y) (`KismetMathLibrary.BreakVector2D` (`self.ScaleMinMax`)))
  (bind _randomstream (`self.RandomStream`))
  (bind _returnvalue (+ (`local.LastLocation`) (`.TotalWidth` (`self.CalculateBookWidth` (`local.CurrentRoll`) (`local.CurrentScale`)))))
  (for _index (range (`self.NumberOfBooks`))
    (set `local.CurrentIndex` _index)
    (set `local.CurrentScale` (`KismetMathLibrary.RandomFloatInRangeFromStream` _scaleminmax_x _scaleminmax_y (`self.RandomStream`)))
    (set `local.currentYaw` (* (`KismetMathLibrary.SelectFloat` 1.0 0.1 (`KismetMathLibrary.RandomBoolWithWeightFromStream` 0.5 _randomstream)) (`KismetMathLibrary.RandomFloatInRangeFromStream` -30.0 30.0 _randomstream)))
    (`|ExecutionSequence`
      (:`then_0`
        (`InstancedStaticMeshComponent.AddInstance` (`self.InstancedStaticMesh`) (`KismetMathLibrary.MakeTransform` (+ (`KismetMathLibrary.MakeVector` 0.0 0.0 _returnvalue) (* (`KismetMathLibrary.GreaterGreater_VectorRotator` (`self.BookSize`) (`KismetMathLibrary.MakeRotator` 90.0 0.0 (`local.currentYaw`))) -0.5)) (`KismetMathLibrary.MakeRotator` 90.0 0.0 (`local.currentYaw`)) (`KismetMathLibrary.Conv_DoubleToVector` (`local.CurrentScale`)))))
      (:`then_1`
        (set `local.LastLocation` _returnvalue)))))

(fn `UserConstructionScript`
  (bind (_returnvalue_min _returnvalue_max) (break `Box` (`StaticMesh.GetBoundingBox` (`StaticMeshComponent.StaticMesh` (`self.InstancedStaticMesh`)))))
  (`KismetMathLibrary.SetRandomStreamSeed` (`self.RandomStream`) (`self.RandomSeed`))
  (set `self.BookSize` (- _returnvalue_max _returnvalue_min))
  (`SceneComponent.SetVisibility` (`self.Spline`) false false)
  (switch `/Game/MedievalHouses/Blueprints/EBookStackType` (`self.StackType`)
    (:`NewEnumerator0`
      (`self.PlaceHorizontalStack`))
    (:`NewEnumerator1`
      (`self.PlaceVerticalStack`))
    (:`NewEnumerator3`
      (`self.PlaceSplineStack`))))