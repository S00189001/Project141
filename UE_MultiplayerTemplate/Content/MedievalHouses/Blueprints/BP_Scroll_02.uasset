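; BP_Scroll_02 is a MedievalHouses prop Blueprint, named for a scroll, that lays out a randomized 3D grid of instanced meshes.
; Its construction script adds one Instanced Static Mesh component and fills it by row, column and height counts and spacing.
; A seeded random stream jitters each instance's position, yaw and uniform scale, though the Y jitter's upper bound reads RandomOffset.X instead of Y.
; The event graph holds only disabled stubs.
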(fn `UserConstructionScript`
  (bind (_randomoffset_x _randomoffset_y) (`KismetMathLibrary.BreakVector2D` (`self.RandomOffset`)))
  (bind _randomoffset_x_2 (`KismetMathLibrary.BreakVector2D` (`self.RandomOffset`)))
  (bind _randomheight (`self.RandomHeight`))
  (bind _randomrotation (`self.RandomRotation`))
  (bind _randomscale (`self.RandomScale`))
  (`KismetMathLibrary.SetRandomStreamSeed` (`self.RandomStream`) (`self.RandomSeed`))
  (bind _returnvalue (`AddComponent|NODE_AddInstancedStaticMeshComponent-0`))
  ;[1 1 1] Rows
  (for _index (range (`self.RowCount`))
    ;[1 1 1] Columns
    (for _index_2 (range (`self.ColumnCount`))
      ;[1 1 1] Height
      (for _index_3 (range (`self.HeightCount`))
        (`InstancedStaticMeshComponent.AddInstance` _returnvalue (`KismetMathLibrary.MakeTransform` (`KismetMathLibrary.MakeVector` (+ (* _index_2 (`self.ColumnSize`)) (`KismetMathLibrary.RandomFloatInRangeFromStream` (* _randomoffset_x_2 -1.0) _randomoffset_x_2 (`self.RandomStream`))) (+ (* _index (`self.RowSize`)) (`KismetMathLibrary.RandomFloatInRangeFromStream` (* _randomoffset_y -1.0) _randomoffset_x (`self.RandomStream`))) (+ (* _index_3 (`self.HeightSize`)) (`KismetMathLibrary.RandomFloatInRangeFromStream` (* _randomheight -1.0) _randomheight (`self.RandomStream`)))) (`KismetMathLibrary.MakeRotator` 0.0 0.0 (`KismetMathLibrary.RandomFloatInRangeFromStream` (* _randomrotation -1.0) _randomrotation (`self.RandomStream`))) (`KismetMathLibrary.Conv_DoubleToVector` (+ (`KismetMathLibrary.RandomFloatInRangeFromStream` (* _randomscale -1.0) _randomscale (`self.RandomStream`)) 1.0))))))))