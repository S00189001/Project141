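; Enemy spawner actor that places EnemyAI_Melee_01 enemies at its root transform, starting on BeginPlay.
; SpawnMob calls itself after Delay nodes, spawning every few seconds while MobsSpawned is below MobsSpawnMax.
; At the cap it rechecks at a much longer interval, but nothing in this Blueprint lowers the count.
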(event `Spawn Mob`
  (if (< (`self.MobsSpawned`) (`self.MobsSpawnMax`))
    (`|SpawnActorFromClass` "/Game/AI/EnemyAI/MeleeAI/EnemyAI_Melee_01/EnemyAI_Melee_01.EnemyAI_Melee_01_C" (`SceneComponent.K2_GetComponentToWorld` (`self.DefaultSceneRoot`)) "Undefined" "OverrideRootScale" null null)
    (`/Engine/EditorBlueprintResources/StandardMacros.IncrementInt` (`self.MobsSpawned`)
      (:`  `
        (`KismetSystemLibrary.Delay` 10.0)
        (`self.Spawn Mob`)))
    (else
      (`KismetSystemLibrary.Delay` 300.0)
      (`self.Spawn Mob`))))

(event `self.ReceiveBeginPlay`
  (`self.Spawn Mob`))

(fn `UserConstructionScript`)