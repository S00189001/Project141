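; Master enemy AI Blueprint that sets up basic stats and can locate the nearest player.
; BeginPlay fills current health from max health and applies the configured walk speed to character movement.
; A Server_FindClosestPlayer event loops over all ThirdPersonCharacter actors and stores the closest one within a fixed starting range, along with its distance.
; Nothing in this graph calls that search or acts on its result.
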(event `self.ReceiveBeginPlay`
  (set `self.CurrentHealth` (`self.MaxHealth`))
  (set `CharacterMovementComponent.MaxWalkSpeed` (`self.MaxWalkSpeed`) (`self.CharacterMovement`)))

(event `Server_FindClosestPlayer`
  ;[1 1 1] Find Closest Player
  (set `self.ClosestPlayerDistance` 2000.0)
  (bind _outactors (`GameplayStatics.GetAllActorsOfClass` "/Game/ThirdPersonCPP/Blueprints/ThirdPersonCharacter.ThirdPersonCharacter_C"))
  (for _array_element _outactors
    (bind _returnvalue (`self.GetDistanceTo` _array_element self))
    (if (< _returnvalue (`self.ClosestPlayerDistance`))
      (set `self.ClosestPlayerDistance` _returnvalue)
      (set `self.ClosestPlayer` _array_element))))

(fn `UserConstructionScript`)